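; Game instance Blueprint with a function that builds a list of selectable screen resolutions as text.
; LoadRes clears the Resolutions array, then queries the supported fullscreen resolutions.
; It keeps only those that meet a minimum width and stores each as a width-by-height string.
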(fn `loadRes`
  (`KismetArrayLibrary.Array_Clear` (`self.Resolutions`))
  (bind _resolutions (`KismetSystemLibrary.GetSupportedFullscreenResolutions`))
  (for _array_element _resolutions
    (bind (_x _y) (break `IntPoint` _array_element))
    (if (>= _x 1024)
      (`KismetArrayLibrary.Array_Add` (`self.Resolutions`) (`self.AppendMultiple` (`KismetStringLibrary.Conv_IntToString` _x) "x" (`KismetStringLibrary.Conv_IntToString` _y)))))
  (return))