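; Player controller that runs the front-end menus: main, play, host, join, spectate and settings screens, plus a background and error popup.
; LeaveCurrentState macro tracks MenuState, hides the outgoing screen and lets each Show event lazily create or reveal its cached widget with UI-only input.
; Host, Join and Spectate have Hide events, but the state switch leaves those cases empty.
; StartGame calls the game instance's LoadRes, then shows the background and main menu.
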(event `Show Spectate Menu`
  (bind _mm_spectate (`self.MM_Spectate`))
  ;[0.3608 1 0.8157] Show Spectate Menu
  (`self.Leave Current State` "NewEnumerator17"
    (:`New State`
      (`/Engine/EditorBlueprintResources/StandardMacros.IsValid` _mm_spectate
        (:`Is Valid`
          (`Widget.SetVisibility` _mm_spectate "Visible"))
        (:`Is Not Valid`
          (bind _returnvalue (`|CreateWidget` "/Game/UI/MainMenus_Blueprints/MM_Spectate.MM_Spectate_C" self))
          (bind _output_get (set `self.MM_Spectate` _returnvalue))
          (`UserWidget.AddToViewport` _output_get 0)))
      (`WidgetBlueprintLibrary.SetInputMode_UIOnlyEx` self null true)
      (set `self.bShowMouseCursor` true))))

(event `Hide Spectate Menu`
  (bind _mm_spectate (`self.MM_Spectate`))
  ;[1 0.01177 0] Hide Spectate Menu
  (`/Engine/EditorBlueprintResources/StandardMacros.IsValid` _mm_spectate
    (:`Is Valid`
      (`Widget.SetVisibility` _mm_spectate "Hidden"))))

(event `Show Join Menu`
  (bind _mm_join (`self.MM_Join`))
  ;[0.3608 1 0.8157] Show Join Menu
  (`self.Leave Current State` "NewEnumerator3"
    (:`New State`
      (`/Engine/EditorBlueprintResources/StandardMacros.IsValid` _mm_join
        (:`Is Valid`
          (`Widget.SetVisibility` _mm_join "Visible"))
        (:`Is Not Valid`
          (bind _returnvalue (`|CreateWidget` "/Game/UI/MainMenus_Blueprints/MM_Join.MM_Join_C" self))
          (bind _output_get (set `self.MM_Join` _returnvalue))
          (`UserWidget.AddToViewport` _output_get 0)))
      (`WidgetBlueprintLibrary.SetInputMode_UIOnlyEx` self null true)
      (set `self.bShowMouseCursor` true))))

(event `Hide Join Menu`
  (bind _mm_join (`self.MM_Join`))
  ;[1 0.01177 0] Hide Join Menu
  (`/Engine/EditorBlueprintResources/StandardMacros.IsValid` _mm_join
    (:`Is Valid`
      (`Widget.SetVisibility` _mm_join "Hidden"))))

(event `Show Host Menu`
  (bind _mm_host (`self.MM_Host`))
  ;[0.3608 1 0.8157] Show Host Menu
  (`self.Leave Current State` "NewEnumerator2"
    (:`New State`
      (`/Engine/EditorBlueprintResources/StandardMacros.IsValid` _mm_host
        (:`Is Valid`
          (`Widget.SetVisibility` _mm_host "Visible"))
        (:`Is Not Valid`
          (bind _returnvalue (`|CreateWidget` "/Game/UI/MainMenus_Blueprints/MM_Host.MM_Host_C" self))
          (bind _output_get (set `self.MM_Host` _returnvalue))
          (`UserWidget.AddToViewport` _output_get 0)))
      (`WidgetBlueprintLibrary.SetInputMode_UIOnlyEx` self null true)
      (set `self.bShowMouseCursor` true))))

(event `Hide Host Menu`
  (bind _mm_host (`self.MM_Host`))
  ;[1 0.01177 0] Hide Host Menu
  (`/Engine/EditorBlueprintResources/StandardMacros.IsValid` _mm_host
    (:`Is Valid`
      (`Widget.SetVisibility` _mm_host "Hidden"))))

(event `Show Play Menu`
  (bind _mm_play (`self.MM_Play`))
  ;[0.3608 1 0.8157] Show Play Menu
  (`self.Leave Current State` "NewEnumerator16"
    (:`New State`
      (`/Engine/EditorBlueprintResources/StandardMacros.IsValid` _mm_play
        (:`Is Valid`
          (`Widget.SetVisibility` _mm_play "Visible"))
        (:`Is Not Valid`
          (bind _returnvalue (`|CreateWidget` "/Game/UI/MainMenus_Blueprints/MM_Play.MM_Play_C" self))
          (bind _output_get (set `self.MM_Play` _returnvalue))
          (`UserWidget.AddToViewport` _output_get 0)))
      (`WidgetBlueprintLibrary.SetInputMode_UIOnlyEx` self null true)
      (set `self.bShowMouseCursor` true))))

(event `Hide Play Menu`
  (bind _mm_play (`self.MM_Play`))
  ;[1 0.01177 0] Hide Play Menu
  (`/Engine/EditorBlueprintResources/StandardMacros.IsValid` _mm_play
    (:`Is Valid`
      (`Widget.SetVisibility` _mm_play "Hidden"))))

(event `Show Video`
  (bind _mm_video (`self.MM_Video`))
  ;[0.3608 1 0.8157] Show Video Settings
  (`self.Leave Current State` "NewEnumerator11"
    (:`New State`
      (`/Engine/EditorBlueprintResources/StandardMacros.IsValid` _mm_video
        (:`Is Valid`
          (`Widget.SetVisibility` _mm_video "Visible"))
        (:`Is Not Valid`
          (bind _returnvalue (`|CreateWidget` "/Game/UI/MainMenus_Blueprints/MM_Video.MM_Video_C" self))
          (bind _output_get (set `self.MM_Video` _returnvalue))
          (`UserWidget.AddToViewport` _output_get 0)))
      (`WidgetBlueprintLibrary.SetInputMode_UIOnlyEx` self null true)
      (set `self.bShowMouseCursor` true))))

(event `Hide Video Settings`
  (bind _mm_video (`self.MM_Video`))
  ;[1 0.01177 0] Hide Video Settings
  (`/Engine/EditorBlueprintResources/StandardMacros.IsValid` _mm_video
    (:`Is Valid`
      (`Widget.SetVisibility` _mm_video "Hidden"))))

(event `Show Audio`
  (bind _mm_audio (`self.MM_Audio`))
  ;[0.3608 1 0.8157] Show Audio Settings
  (`self.Leave Current State` "NewEnumerator10"
    (:`New State`
      (`/Engine/EditorBlueprintResources/StandardMacros.IsValid` _mm_audio
        (:`Is Valid`
          (`Widget.SetVisibility` _mm_audio "Visible"))
        (:`Is Not Valid`
          (bind _returnvalue (`|CreateWidget` "/Game/UI/MainMenus_Blueprints/MM_Audio.MM_Audio_C" self))
          (bind _output_get (set `self.MM_Audio` _returnvalue))
          (`UserWidget.AddToViewport` _output_get 0)))
      (`WidgetBlueprintLibrary.SetInputMode_UIOnlyEx` self null true)
      (set `self.bShowMouseCursor` true))))

(event `Hide Audio Settings`
  (bind _mm_audio (`self.MM_Audio`))
  ;[1 0.01177 0] Hide Audio
  (`/Engine/EditorBlueprintResources/StandardMacros.IsValid` _mm_audio
    (:`Is Valid`
      (`Widget.SetVisibility` _mm_audio "Hidden"))))

(event `Show Controls`
  (bind _mm_controls (`self.MM_Controls`))
  ;[0.3608 1 0.8157] Show Control Settings
  (`self.Leave Current State` "NewEnumerator5"
    (:`New State`
      (`/Engine/EditorBlueprintResources/StandardMacros.IsValid` _mm_controls
        (:`Is Valid`
          (`Widget.SetVisibility` _mm_controls "Visible"))
        (:`Is Not Valid`
          (bind _returnvalue (`|CreateWidget` "/Game/UI/MainMenus_Blueprints/MM_Controls.MM_Controls_C" self))
          (bind _output_get (set `self.MM_Controls` _returnvalue))
          (`UserWidget.AddToViewport` _output_get 0)))
      (`WidgetBlueprintLibrary.SetInputMode_UIOnlyEx` self null true)
      (set `self.bShowMouseCursor` true))))

(event `Hide Control Settings`
  (bind _mm_controls (`self.MM_Controls`))
  ;[1 0.01177 0] Hide Control Settings
  (`/Engine/EditorBlueprintResources/StandardMacros.IsValid` _mm_controls
    (:`Is Valid`
      (`Widget.SetVisibility` _mm_controls "Hidden"))))

(event `Show Settings`
  (bind _mm_settingstab (`self.MM_SettingsTab`))
  ;[0.3608 1 0.8157] Show Settings
  (`self.Leave Current State` "NewEnumerator4"
    (:`New State`
      (`/Engine/EditorBlueprintResources/StandardMacros.IsValid` _mm_settingstab
        (:`Is Valid`
          (`Widget.SetVisibility` _mm_settingstab "Visible"))
        (:`Is Not Valid`
          (bind _returnvalue (`|CreateWidget` "/Game/UI/MainMenus_Blueprints/W_Settings.W_Settings_C" self))
          (bind _output_get (set `self.MM_SettingsTab` _returnvalue))
          (`UserWidget.AddToViewport` _output_get 0)))
      (`WidgetBlueprintLibrary.SetInputMode_UIOnlyEx` self null true)
      (set `self.bShowMouseCursor` true))))

(event `Hide Settings`
  (bind _mm_settingstab (`self.MM_SettingsTab`))
  ;[1 0.01492 0] Hide Settings
  (`/Engine/EditorBlueprintResources/StandardMacros.IsValid` _mm_settingstab
    (:`Is Valid`
      (`Widget.SetVisibility` _mm_settingstab "Hidden"))))

(event `Show Main Menu`
  (bind _mm_main (`self.MM_Main`))
  ;[0.3608 1 0.8157] Show Main Menu
  (`self.Leave Current State` "NewEnumerator1"
    (:`New State`
      (`/Engine/EditorBlueprintResources/StandardMacros.IsValid` _mm_main
        (:`Is Valid`
          (`Widget.SetVisibility` _mm_main "Visible"))
        (:`Is Not Valid`
          (bind _returnvalue (`|CreateWidget` "/Game/UI/MainMenus_Blueprints/MM_Main.MM_Main_C" self))
          (bind _output_get (set `self.MM_Main` _returnvalue))
          (`UserWidget.AddToViewport` _output_get 0)))
      (`WidgetBlueprintLibrary.SetInputMode_UIOnlyEx` self null true)
      (set `self.bShowMouseCursor` true))))

(event `Hide Main Menu`
  (bind _mm_main (`self.MM_Main`))
  ;[1 0.03007 0] Hide Main Menu
  (`/Engine/EditorBlueprintResources/StandardMacros.IsValid` _mm_main
    (:`Is Valid`
      (`Widget.SetVisibility` _mm_main "Hidden"))))

(event `Show_Background`
  (bind _mm_background (`self.MM_Background`))
  ;[0.3608 1 0.8157] Show Background
  (`/Engine/EditorBlueprintResources/StandardMacros.IsValid` _mm_background
    (:`Is Valid`
      (`Widget.SetVisibility` _mm_background "Visible"))
    (:`Is Not Valid`
      (bind _returnvalue (`|CreateWidget` "/Game/UI/MainMenus_Blueprints/MM_Background.MM_Background_C" (`GameplayStatics.GetPlayerController` 0)))
      (bind _output_get (set `self.MM_Background` _returnvalue))
      (`UserWidget.AddToViewport` _output_get 0))))

(event `End Game`
  ;[0.3608 1 0.8157] End Game
  (`KismetSystemLibrary.ExecuteConsoleCommand` "quit"))

(event `Start Over`
  ;[1 1 1] Restart Game
  (`self.Start Game`))

(event `Restart_Over`
  ;[1 1 1] Back to Main Menu
  (`GameplayStatics.OpenLevel` "Menus"))

(event `DESTROY_ERROR_MSG`
  (bind _error_msg (`self.Error_MSG`))
  ;[1 1 1] Destroy Error MSG
  (`/Engine/EditorBlueprintResources/StandardMacros.IsValid` _error_msg
    (:`Is Valid`
      (`Widget.RemoveFromParent` _error_msg)
      (`self.Restart_Over`))))

(event `Show Error MSG`
  (params (`Error Text` :type Text))
  ;[1 1 1] Show Error MSG
  (`/Engine/EditorBlueprintResources/StandardMacros.IsValid` (`self.Error_MSG`)
    (:`Is Not Valid`
      (bind _returnvalue (`|CreateWidget` "/Game/UI/MainMenus_Blueprints/Error_MSG_WG.Error_MSG_WG_C" self `Error Text`))
      (bind _output_get (set `self.Error_MSG` _returnvalue))
      (`UserWidget.AddToViewport` _output_get 0))))

(event `Start Game`
  ;[1 1 1] Start Game
  (bind _asgame_instance_ic (cast `/Game/Blueprints/GameInstance_IC` (`GameplayStatics.GetGameInstance`)))
  (`/Game/Blueprints/GameInstance_IC.loadRes` _asgame_instance_ic)
  (`self.Leave Current State` "NewEnumerator0"
    (:`New State`
      _)
    (:`Same State`
      _))
  (`self.Show_Background`)
  (`self.Show Main Menu`))

(fn `UserConstructionScript`)